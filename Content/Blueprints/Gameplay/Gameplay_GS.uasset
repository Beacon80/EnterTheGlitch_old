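; Gameplay game state (GS) that tracks the three playable siblings, Jenn, Ner and Rick, and the level's collectibles.
; Maps populate the sibling array, which player controllers cycle with wrap-around to possess unclaimed siblings, updating each sibling's stored player name.
; Collectibles share one flag array indexed through GetSuperIndex, which also increments the coin count; only coins are counted so far.
; Debug events print collected coins and powerup container contents.
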(event `PopulateSiblingArray`
  (bind _siblings (`self.Siblings`))
  ;[1 1 1] Creates an array with the siblings. Should be called from each map's blueprint
  (`KismetArrayLibrary.Array_Clear` _siblings)
  (bind _returnvalue (`GameplayStatics.GetActorOfClass` "/Game/Blueprints/Characters/Jenn.Jenn_C"))
  (bind _returnvalue_2 (`KismetArrayLibrary.Array_Add` _siblings _returnvalue))
  (set `self.JennIndex` _returnvalue_2)
  (bind _returnvalue_3 (`GameplayStatics.GetActorOfClass` "/Game/Blueprints/Characters/Ner.Ner_C"))
  (bind _returnvalue_4 (`KismetArrayLibrary.Array_Add` _siblings _returnvalue_3))
  (set `self.NerIndex` _returnvalue_4)
  (bind _returnvalue_5 (`GameplayStatics.GetActorOfClass` "/Game/Blueprints/Characters/Rick.Rick_C"))
  (bind _returnvalue_6 (`KismetArrayLibrary.Array_Add` _siblings _returnvalue_5))
  (set `self.RickIndex` _returnvalue_6))

(event `DisplayAllContainers`
  (bind _outactors (`GameplayStatics.GetAllActorsOfClass` "/Game/Blueprints/Objects/PowerupContainers/PowerupContainer.PowerupContainer_C"))
  (for _array_element _outactors
    (switch `/Game/Blueprints/PowerUp/E_Powerups` (`/Game/Blueprints/PowerUp/Powerup.PowerupType` (`/Game/Blueprints/Objects/PowerupContainers/PowerupContainer.HeldPowerup` _array_element))
      (:`NewEnumerator2`
        (`KismetSystemLibrary.PrintString` "Empty"))
      (:`NewEnumerator0`
        (`KismetSystemLibrary.PrintString` "doublejump"))
      (:`NewEnumerator1`
        (`KismetSystemLibrary.PrintString` "Glide"))
      (:`NewEnumerator3`
        (`KismetSystemLibrary.PrintString` "RunningShoes")))))

(event `InitializeCollectibles`
  (bind _allcollectibleflags (`self.AllCollectibleFlags`))
  ;[1 1 1] Initialize the collectibles
  (bind _output_get (set `self.TotalCollectibles` (+ (`self.TotalCoins`) 0)))
  (`KismetArrayLibrary.Array_Resize` _allcollectibleflags _output_get)
  (for _index (range (+ _output_get 1))
    (`KismetArrayLibrary.Array_Set` _allcollectibleflags _index))
  (set `self.ZeroIndexCoins` 0))

(event `CollectCollectible`
  (params (Type :type "/Game/Blueprints/Objects/Collectibles/E_Collectibles Enum" :default "NewEnumerator0") (Index :type Integer))
  (bind _superindex (`self.GetSuperIndex` Type Index))
  (`KismetArrayLibrary.Array_Set` (`self.AllCollectibleFlags`) _superindex true))

(event `PrintCollectibles`
  (`KismetSystemLibrary.PrintString` (`KismetStringLibrary.Concat_StrStr` (`KismetStringLibrary.Conv_IntToString` (`self.CollectedCoins`)) " collected out of " (`KismetStringLibrary.Conv_IntToString` (`self.TotalCoins`))) true true (struct :`R` 0.963507 :`G` 1.0 :`A` 1.0) 5.0)
  (for _index (range (`self.ZeroIndexCoins`) (+ (`self.TotalCoins`) 1))
    (if (`|GetArrayItem` (`self.AllCollectibleFlags`) _index)
      (`KismetSystemLibrary.PrintString` (`KismetStringLibrary.Conv_IntToString` _index) true true (struct :`R` 0.963507 :`G` 1.0 :`A` 1.0) 5.0))))

(fn `GetAllSibConNames`
  (returns (JennConName :type Text) (NerConName :type Text) (RickConName :type Text))
  (return (`self.JennConName`) (`self.NerConName`) (`self.RickConName`)))

(fn `GetJenn`
  (returns (Jenn :type "/Game/Blueprints/Characters/0_Sibling Object Reference"))
  (return (`|GetArrayItem` (`self.Siblings`) (`self.JennIndex`))))

(fn `GetNer`
  (returns (Ner :type "/Game/Blueprints/Characters/0_Sibling Object Reference"))
  (return (`|GetArrayItem` (`self.Siblings`) (`self.NerIndex`))))

(fn `GetNextAvailableSibling`
  (params (SiblingIndex :type Integer) (Right :type Boolean))
  (returns (Sibling :type "/Game/Blueprints/Characters/0_Sibling Object Reference") (Success :type Boolean))
  (locals (IndexMod :type Integer) (Index :type Integer))
  (set `local.Index` SiblingIndex)
  (if Right
    (set `local.IndexMod` 1)
    (else
      (set `local.IndexMod` -1)))
  (bind _retval (`self.WrapIndex` (+ (`local.Index`) (`local.IndexMod`))))
  (bind _output_get (set `local.Index` _retval))
  (bind _output (`|GetArrayItem` (`self.Siblings`) _output_get))
  (if (`/Game/Blueprints/Characters/0_Sibling.IsPossessed` _output)
    (bind _retval_2 (`self.WrapIndex` (+ (`local.Index`) (`local.IndexMod`))))
    (bind _output_get_2 (set `local.Index` _retval_2))
    (bind _output_2 (`|GetArrayItem` (`self.Siblings`) _output_get_2))
    (if (`/Game/Blueprints/Characters/0_Sibling.IsPossessed` _output_2)
      (return null false)
      (else
        (return _output_2 true)))
    (else
      (return _output true))))

(fn `GetRick`
  (returns (Rick :type "/Game/Blueprints/Characters/0_Sibling Object Reference"))
  (return (`|GetArrayItem` (`self.Siblings`) (`self.RickIndex`))))

(fn `GetSibConName`
  (params (Sibling :type "/Game/Blueprints/Characters/0_Sibling Object Reference"))
  (returns (SibConName :type Text))
  (bind _returnvalue (`Pawn.GetController` Sibling))
  (if (`KismetSystemLibrary.IsValid` _returnvalue)
    (bind _asgameplay_pc (cast `/Game/Blueprints/Gameplay/Gameplay_PC` _returnvalue)
      (:`then`
        (return (`.MyplayerName_19_E7F6C02C4EDEABB78B2B6780C19B040E` (break `/Game/Blueprints/AllLevels/PlayerInfo` (`/Game/Blueprints/Gameplay/Gameplay_PC.PlayerSettings` _asgameplay_pc)))))
      (:`CastFailed`
        _)))
  (return ""))

(fn `GetSiblingByNumber`
  (params (SiblingIndex :type Integer))
  (returns (Sibling :type "/Game/Blueprints/Characters/0_Sibling Object Reference"))
  (return (`|GetArrayItem` (`self.Siblings`) SiblingIndex)))

(fn `GetSuperIndex`
  (params (Type :type "/Game/Blueprints/Objects/Collectibles/E_Collectibles Enum" :default "NewEnumerator0") (Index :type Integer))
  (returns (SuperIndex :type Integer))
  (switch `/Game/Blueprints/Objects/Collectibles/E_Collectibles` Type
    (:`NewEnumerator0`
      (`/Engine/EditorBlueprintResources/StandardMacros.IncrementInt` (`self.CollectedCoins`)
        (:`  `
          (return (+ Index (`self.ZeroIndexCoins`))))))))

(fn `Possess Sibling`
  (params (OldSibling :type "/Game/Blueprints/Characters/0_Sibling Object Reference") (NewSibling :type "/Game/Blueprints/Characters/0_Sibling Object Reference") (PC :type "/Game/Blueprints/Gameplay/Gameplay_PC Object Reference"))
  (returns (Success :type Boolean))
  (if (`/Game/Blueprints/Characters/0_Sibling.IsPossessed` NewSibling)
    (return false)
    (else
      (set `/Game/Blueprints/Characters/0_Sibling.IsPossessed` true NewSibling)
      (`self.UpdateSibConName` (`.MyplayerName_19_E7F6C02C4EDEABB78B2B6780C19B040E` (break `/Game/Blueprints/AllLevels/PlayerInfo` (`/Game/Blueprints/Gameplay/Gameplay_PC.PlayerSettings` PC))) NewSibling)
      (set `/Game/Blueprints/Gameplay/Gameplay_PC.LastSibling` (`/Game/Blueprints/Characters/0_Sibling.SibIndex` NewSibling) PC)
      (`self.UnpossessSibling` OldSibling)
      (`self.UpdateSibConName` "" OldSibling)
      (`Controller.Possess` PC NewSibling)
      (return true))))

(fn `RefreshSibConNames`
  (bind _jenn (`self.GetJenn`))
  (bind _sibconname (`self.GetSibConName` _jenn))
  (set `self.JennConName` _sibconname)
  (bind _ner (`self.GetNer`))
  (bind _sibconname_2 (`self.GetSibConName` _ner))
  (set `self.NerConName` _sibconname_2)
  (bind _rick (`self.GetRick`))
  (bind _sibconname_3 (`self.GetSibConName` _rick))
  (set `self.RickConName` _sibconname_3))

(fn `UpdateSibConName`
  (params (ConName :type Text) (Sibling :type "/Game/Blueprints/Characters/0_Sibling Object Reference"))
  (if (`KismetSystemLibrary.IsValid` Sibling)
    (switch `/Game/Blueprints/Characters/E_Sibling` (`/Game/Blueprints/Characters/0_Sibling.WhichSib?` Sibling)
      (:`NewEnumerator0`
        (set `self.JennConName` ConName))
      (:`NewEnumerator1`
        (set `self.NerConName` ConName))
      (:`NewEnumerator2`
        (set `self.RickConName` ConName)))))

(fn `UserConstructionScript`)

(fn `WrapIndex`
  (params (Index :type Integer))
  (returns (RetVal :type Integer))
  (if (> Index 2)
    (return 0)
    (elif (< Index 0)
      (return 2)
      (else
        (return Index)))))